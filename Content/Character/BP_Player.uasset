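; Player character Blueprint with Enhanced Input movement, footstep audio, three abilities and HP that reloads the level at zero.
; Attack swings the sword and box-traces damage, E box-traces from the camera for damage plus explosions, and Q line-traces to spawn a healing zone.
; DoOnce gates throttle actions, with Timelines resetting them and driving per-ability cooldown floats.
; Curar adds clamped health, and key 1 plays a cosmetic sword gesture.
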(event `self.ReceiveBeginPlay`
  ; begin play
  (`EnhancedInputSubsystemInterface.AddMappingContext` (pcsubsystem `EnhancedInputLocalPlayerSubsystem` (`GameplayStatics.GetPlayerController` 0)) "/Game/Character/Input/IMC_Controles.IMC_Controles" 0 (struct))
  (bind _returnvalue (`GameplayStatics.GetActorOfClass` "/Game/Character/Peronsaje_Q/BP_AuraLuzSanacion.BP_AuraLuzSanacion_C"))
  (set `self.AuraLuzQ` _returnvalue))

(event `self.ReceiveAnyDamage`
  (params (Damage :type "Float (single-precision)") (DamageType :type "DamageType Object Reference") (InstigatedBy :type "Controller Object Reference") (DamageCauser :type "Actor Object Reference"))
  ; RECIVIR DAÑo
  (`/Engine/EditorBlueprintResources/StandardMacros.DoOnce` false :!label _label
    (:`Completed`
      (bind _output_get (set `self.HP_Player` (- (`self.HP_Player`) (`KismetMathLibrary.FClamp` Damage 0.0 10.0))))
      (if (== _output_get 0.0)
        ; CUANDO SE MUERE EL PANA
        ;; Reinicio de nivel
        (bind _returnvalue (`GameplayStatics.GetCurrentLevelName` true))
        (`GameplayStatics.OpenLevel` (`KismetStringLibrary.Conv_StringToName` _returnvalue))
        (else
          (`KismetSystemLibrary.PrintString` (`KismetStringLibrary.Conv_DoubleToString` _output_get))
          (`KismetSystemLibrary.Delay` 0.2)
          (goto _label :!via `Reset`))))))

(event `EnhancedInput|/Game/Character/Input/Actions/IA_Ataque`
  (params (ActionValue :type Boolean) (ElapsedSeconds :type "Float (double-precision)") (TriggeredSeconds :type "Float (double-precision)") (InputAction :type "InputAction Object Reference" :default "/Game/Character/Input/Actions/IA_Ataque.IA_Ataque"))
  (bind _mesh (`self.Mesh`))
  (bind _returnvalue (`SceneComponent.K2_GetComponentLocation` _mesh))
  ; ATAQUE CLICK IZQUIERDO
  (:`Started`
    (`/Engine/EditorBlueprintResources/StandardMacros.DoOnce` false :!label _label_2
      (:`Completed`
        (`self.MoverEspada`)
        (bind (_outhits _returnvalue_2) (`KismetSystemLibrary.BoxTraceMultiForObjects` _returnvalue (+ _returnvalue (* (`SceneComponent.GetForwardVector` _mesh) 300.0)) (50.0 50.0 50.0) (struct) (`|MakeArray` "ObjectTypeQuery3" :!type "EObjectTypeQuery Enum") false (`|MakeArray` self :!type "Actor Object Reference")))
        (`GameplayStatics.PlaySound2D` "/Game/Character/art/_espada-ataque-2._espada-ataque-2" 1.0 1.0 0.0 null null)
        (for _array_element _outhits
          (if _returnvalue_2
            (`GameplayStatics.ApplyDamage` (`.HitActor` (`GameplayStatics.BreakHitResult` _array_element)) 1.0)
            (bind (_direction _newtrack_0) (`Timeline|Timeline_2` :!via `PlayFromStart` :!label _label_3)
              (:`Update`
                (set `self.FloatAtack` (`KismetMathLibrary.Lerp` 0.0 1000.0 _newtrack_0)))
              (:`Finished`
                (goto _label_2 :!via `Reset`)))))
        (goto _label_3 :!via `PlayFromStart`)))))

(event `MoverEspada`
  (bind _espadaorigin (`self.espadaOrigin`))
  ; ANIMACION DE ESPADA
  (`/Engine/EditorBlueprintResources/StandardMacros.DoOnce` false :!label _label_4
    (:`Completed`
      (bind (_direction _newtrack_0) (`Timeline|espda` :!via `PlayFromStart`)
        (:`Update`
          (`SceneComponent.K2_SetRelativeRotation` _espadaorigin (`KismetMathLibrary.RLerp` (struct) (struct :`Pitch` -70.0) _newtrack_0) false false)
          (`SceneComponent.K2_SetRelativeLocation` _espadaorigin (`KismetMathLibrary.VLerp` (37.933281 23.960878 -23.884631) (56.228692 23.960878 -37.250387) _newtrack_0) true false))
        (:`Finished`
          (goto _label_4 :!via `Reset`))))))

(event `SonidoGuiño`
  (`GameplayStatics.PlaySound2D` null 1.0 1.0 0.0 null null)
  (`GameplayStatics.PlaySound2D` "/Game/Character/_espada-contra-escudo1._espada-contra-escudo1" 1.0 1.0 0.0 null null))

(event `EnhancedInput|/Game/Character/Input/Actions/IA_Q`
  (params (ActionValue :type Boolean) (ElapsedSeconds :type "Float (double-precision)") (TriggeredSeconds :type "Float (double-precision)") (InputAction :type "InputAction Object Reference" :default "/Game/Character/Input/Actions/IA_Q.IA_Q"))
  (bind _origenq (`self.origenQ`))
  (bind _returnvalue (`SceneComponent.K2_GetComponentLocation` _origenq))
  ; LUZ CON LA TECLA Q
  (:`Started`
    (`/Engine/EditorBlueprintResources/StandardMacros.DoOnce` false :!label _label_5
      (:`Completed`
        (bind (_outhit _returnvalue_2) (`KismetSystemLibrary.LineTraceSingle` _returnvalue (+ _returnvalue (* (`SceneComponent.GetForwardVector` _origenq) 1000.0)) "TraceTypeQuery1"))
        (if _returnvalue_2
          (`|SpawnActorFromClass` "/Game/Features/BP_ZonaCuracion.BP_ZonaCuracion_C" (`KismetMathLibrary.MakeTransform` (`.Location` (`GameplayStatics.BreakHitResult` _outhit))) "Undefined" "MultiplyWithRoot" null null)
          (bind (_direction _newtrack_0) (`Timeline|Timeline_0` :!via `PlayFromStart`)
            (:`Update`
              (bind _output_get (set `self.FloatQ` (`KismetMathLibrary.Lerp` 0.0 1000.0 _newtrack_0))))
            (:`Finished`
              (goto _label_5 :!via `Reset`))))))))

(event `Key|One`
  (params (Key :type "Key Structure"))
  ; guiño tin tin tinnn
  (:`Pressed`
    (`/Engine/EditorBlueprintResources/StandardMacros.DoOnce` false :!label _label_6
      (:`Completed`
        (`self.SonidoGuiño`)
        (bind (_direction _newtrack_0) (`Timeline|Timeline` :!via `PlayFromStart`)
          (:`Update`
            (`SceneComponent.K2_SetRelativeRotation` (`self.espadaOrigin`) (`KismetMathLibrary.RLerp` (struct) (struct :`Roll` -60.0) _newtrack_0) false false))
          (:`Finished`
            (goto _label_6 :!via `Reset`)))))))

(event `EnhancedInput|/Game/Character/Input/Actions/IA_E`
  (params (ActionValue :type Boolean) (ElapsedSeconds :type "Float (double-precision)") (TriggeredSeconds :type "Float (double-precision)") (InputAction :type "InputAction Object Reference" :default "/Game/Character/Input/Actions/IA_E.IA_E"))
  (bind _camera (`self.Camera`))
  (bind _returnvalue (`SceneComponent.K2_GetComponentLocation` _camera))
  ; RANGO CON LA TECLA E
  (:`Started`
    (`/Engine/EditorBlueprintResources/StandardMacros.DoOnce` false :!label _label_7
      (:`Completed`
        (bind (_outhits _returnvalue_2) (`KismetSystemLibrary.BoxTraceMultiForObjects` _returnvalue (+ _returnvalue (* (`SceneComponent.GetForwardVector` _camera) 1300.0)) (10.0 30.0 400.0) (struct) (`|MakeArray` "ObjectTypeQuery3" "ObjectTypeQuery1" "ObjectTypeQuery2" "ObjectTypeQuery4" "ObjectTypeQuery5" :!type "EObjectTypeQuery Enum") false (`|MakeArray` self :!type "Actor Object Reference") "None" true (struct :`R` 1.0 :`A` 1.0) (struct :`G` 1.0 :`A` 1.0) 0.5))
        (for _array_element _outhits
          (if _returnvalue_2
            (bind (_bblockinghit _binitialoverlap _time _distance _location _impactpoint _normal _impactnormal _physmat _hitactor) (`GameplayStatics.BreakHitResult` _array_element))
            (`GameplayStatics.ApplyDamage` _hitactor 1.0))
          (`self.Explosion` :!label _label_8)
          (`|SpawnActorFromClass` "/Game/Character/Personaje_E/BP_Explosion.BP_Explosion_C" (`KismetMathLibrary.MakeTransform` _impactpoint) "Undefined" "MultiplyWithRoot" null null)
          (bind (_direction _newtrack_0) (`Timeline|Timeline_1` :!via `PlayFromStart`)
            (:`Update`
              (bind _output_get (set `self.FloatE` (`KismetMathLibrary.Lerp` 0.0 1000.0 _newtrack_0))))
            (:`Finished`
              (goto _label_7 :!via `Reset`))))
        (goto _label_8)))))

(event `Explosion`
  (bind _pixil_frame_0_sprite (`self.pixil-frame-0_Sprite`))
  ; ExplosionFeedack
  (`SceneComponent.SetHiddenInGame` _pixil_frame_0_sprite false false)
  (`KismetSystemLibrary.Delay` 0.1)
  (`SceneComponent.SetHiddenInGame` _pixil_frame_0_sprite true false))

(event `EnhancedInput|/Game/Character/Input/Actions/IA_Mirar`
  (params (ActionValue :type "Vector2D Structure") (ElapsedSeconds :type "Float (double-precision)") (TriggeredSeconds :type "Float (double-precision)") (InputAction :type "InputAction Object Reference" :default "/Game/Character/Input/Actions/IA_Mirar.IA_Mirar"))
  ; sistema de movimiento
  (:`Triggered`
    (`self.Mirar` ActionValue_X ActionValue_Y)))

(event `EnhancedInput|/Game/Character/Input/Actions/IA_Saltar`
  (params (ActionValue :type Boolean) (ElapsedSeconds :type "Float (double-precision)") (TriggeredSeconds :type "Float (double-precision)") (InputAction :type "InputAction Object Reference" :default "/Game/Character/Input/Actions/IA_Saltar.IA_Saltar"))
  ; SALTAR
  (:`Started`
    (`self.Jump`)))

(event `EnhancedInput|/Game/Character/Input/Actions/IA_Moverse`
  (params (ActionValue :type "Vector2D Structure") (ElapsedSeconds :type "Float (double-precision)") (TriggeredSeconds :type "Float (double-precision)") (InputAction :type "InputAction Object Reference" :default "/Game/Character/Input/Actions/IA_Moverse.IA_Moverse"))
  ; sistema de movimiento
  (:`Triggered`
    (`self.Moverse` ActionValue_X ActionValue_Y))
  (:`Started`
    (bind _returnvalue (`KismetSystemLibrary.K2_SetTimerDelegate` (delegate `SonarPaso`) 0.3 true)))
  (:`Completed`
    (`KismetSystemLibrary.K2_ClearAndInvalidateTimerHandle` _returnvalue)))

(event `SonarPaso`
  ; sistema de movimiento
  (`GameplayStatics.PlaySound2D` "/Game/Character/art/_pasos-1_Cue._pasos-1_Cue" 1.0 1.0 0.0 null null))

(fn `Curar`
  (params (Cantidad :type "Float (double-precision)"))
  (bind _output_get (set `self.HP_Player` (`KismetMathLibrary.FClamp` (+ (`self.HP_Player`) Cantidad) 0.0 (`self.HP_Max_Player`)))))

(fn `Mirar`
  (params (Yaw :type "Float (double-precision)") (Pitch :type "Float (double-precision)"))
  (`self.AddControllerYawInput` Yaw)
  (`self.AddControllerPitchInput` Pitch))

(fn `Moverse`
  (params (`Izquierda/Derecha` :type "Float (double-precision)") (`Frente/Atras` :type "Float (double-precision)"))
  (`self.AddMovementInput` (`self.GetActorRightVector`) `Izquierda/Derecha`)
  (`self.AddMovementInput` (`self.GetActorForwardVector`) `Frente/Atras`))

(fn `UserConstructionScript`)