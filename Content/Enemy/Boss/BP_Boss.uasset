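; Boss enemy that faces the player, chases when activated and registers as a level objective through BPI_LevelManager.
; Sphere overlap launches and damages the player, while looping timers fire projectiles at distant players and alternately spawn melee and ranged minions up to a cap.
; Damage is clamped per hit and throttled by a resetting DoOnce.
; At zero HP it shows the dead visual, completes the objective and returns to MainMenu.
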(event `self.ReceiveTick`
  (params (DeltaSeconds :type "Float (single-precision)"))
  ; Mover Hacia Jugador
  (`self.K2_SetActorRotation` (`KismetMathLibrary.FindLookAtRotation` (`self.K2_GetActorLocation`) (`self.K2_GetActorLocation` (`self.Player`))))
  (if (`self.ActivateMove`)
    (`|AIMoveTo` self (0.0 0.0 0.0) (`self.Player`) 100.0)))

(event `self.Sphere.OnComponentBeginOverlap`
  (params (OverlappedComponent :type "PrimitiveComponent Object Reference") (OtherActor :type "Actor Object Reference") (OtherComp :type "PrimitiveComponent Object Reference") (OtherBodyIndex :type Integer) (bFromSweep :type Boolean) (SweepResult :type "HitResult Structure (by ref)"))
  (bind _returnvalue (`GameplayStatics.GetPlayerCharacter` 0))
  ; Ataque Melee
  (if (== OtherActor _returnvalue)
    (set `self.bJugadorEnMelee` false)
    (`self.LaunchCharacter` _returnvalue (10.0 10.0 50.0) false false)
    (`GameplayStatics.ApplyDamage` _returnvalue (`self.DanoMelee`))))

(event `SpawnHit`
  (`NiagaraFunctionLibrary.SpawnSystemAtLocation` "/Game/SlashTrail_SoftTofu/Niagara/Dark/NS_Hit_Dark_Once.NS_Hit_Dark_Once" (`SceneComponent.K2_GetComponentLocation` (`self.IdleBoss`)))
  (`GameplayStatics.PlaySound2D` "/Game/Character/art/_impacto._impacto" 1.0 1.0 0.0 null null))

(event `self.ReceiveAnyDamage`
  (params (Damage :type "Float (single-precision)") (DamageType :type "DamageType Object Reference") (InstigatedBy :type "Controller Object Reference") (DamageCauser :type "Actor Object Reference"))
  (`/Engine/EditorBlueprintResources/StandardMacros.DoOnce` false :!label _label
    (:`Completed`
      (`self.SpawnHit`)
      (bind _output_get (set `self.HP` (- (`self.HP`) (`KismetMathLibrary.FClamp` Damage))))
      (`KismetSystemLibrary.PrintString` (`KismetStringLibrary.Conv_DoubleToString` _output_get))
      (if (== _output_get 0.0)
        (`SceneComponent.SetHiddenInGame` (`self.IdleBoss`) true false)
        (`SceneComponent.SetHiddenInGame` (`self.DeadBoss`) false false)
        (`KismetSystemLibrary.Delay` 1.0)
        (`GameplayStatics.PlaySound2D` "/Game/Character/art/saucillator_20260725_125954.saucillator_20260725_125954" 1.0 1.0 0.0 null null)
        (bind _outactors (`GameplayStatics.GetAllActorsWithInterface` "/Game/Features/LevelManager/BPI_LevelManager.BPI_LevelManager_C"))
        (message `/Game/Features/LevelManager/BPI_LevelManager.ObjectiveCompleted` (`|GetArrayItem` _outactors))
        (`KismetSystemLibrary.PrintString` "GANASTEEE")
        (`KismetSystemLibrary.Delay` 5.0)
        (`GameplayStatics.OpenLevel` "MainMenu")
        (`self.K2_DestroyActor`)
        (else
          (`KismetSystemLibrary.Delay` 0.2)
          (goto _label :!via `Reset`))))))

(event `self.ReceiveBeginPlay`
  (bind _outactors (`GameplayStatics.GetAllActorsWithInterface` "/Game/Features/LevelManager/BPI_LevelManager.BPI_LevelManager_C"))
  (message `/Game/Features/LevelManager/BPI_LevelManager.ObjectiveRegistered` (`|GetArrayItem` _outactors))
  (`|ExecutionSequence`
    (:`then_0`
      (bind _returnvalue (`GameplayStatics.GetActorOfClass` "/Game/Character/BP_Player.BP_Player_C"))
      (set `self.Player` _returnvalue)
      (`KismetSystemLibrary.K2_SetTimerDelegate` (delegate `IntentarDisparo`) 3.0 true)
      (set `self.TimerHandle_Disparo` (struct)))
    (:`then_1`
      (`KismetSystemLibrary.K2_SetTimerDelegate` (delegate `spawnearMinion`) (`KismetMathLibrary.RandomFloatInRange` 3.0 7.0) true))))

(event `IntentarDisparo`
  (`GameplayStatics.PlaySoundAtLocation` "/Game/Character/art/_risa-2_Cue._risa-2_Cue" (`self.K2_GetActorLocation`) (struct) 1.0 1.0 0.0 "/Game/SlashTrail_SoftTofu/Resource/Audio/SA_Attenuation_Middle.SA_Attenuation_Middle" null null null)
  (if (> (`self.GetDistanceTo` (`GameplayStatics.GetPlayerPawn` 0)) (`self.RangoMelee`))
    (if (< (`self.GetDistanceTo` (`self.Player`)) 3000.0)
      (`|SpawnActorFromClass` "/Game/Enemy/enemyCharacter/BP_Proyectil.BP_Proyectil_C" (`KismetMathLibrary.MakeTransform` (`self.K2_GetActorLocation`) (`KismetMathLibrary.FindLookAtRotation` (`self.K2_GetActorLocation`) (`self.K2_GetActorLocation` (`GameplayStatics.GetPlayerPawn` 0))) (3.0 3.0 3.0)) "Undefined" "MultiplyWithRoot" null null))))

(event `spawnearMinion`
  (bind (_arrayindex _arrayelement) (`/Engine/EditorBlueprintResources/StandardMacros.ReverseForEachLoop` (`self.SpawnedEnemies`))
    (:`LoopBody`
      (`/Engine/EditorBlueprintResources/StandardMacros.IsValid` _arrayelement
        (:`Is Not Valid`
          (`KismetArrayLibrary.Array_Remove` (`self.SpawnedEnemies`) _arrayindex))))
    (:`Completed`
      (if (< (`KismetArrayLibrary.Array_Length` (`self.SpawnedEnemies`)) 10)
        (`/Engine/EditorBlueprintResources/StandardMacros.FlipFlop`
          (:`A`
            (bind _returnvalue (`|SpawnActorFromClass` "/Game/Enemy/enemyCharacter/BP_Enemy.BP_Enemy_C" (`SceneComponent.K2_GetComponentToWorld` (`self.spawn1`)) "Undefined" "MultiplyWithRoot" null null))
            (`KismetArrayLibrary.Array_Add` (`self.SpawnedEnemies`) _returnvalue))
          (:`B`
            (bind _returnvalue_2 (`|SpawnActorFromClass` "/Game/Enemy/enemyCharacter/BP_EnemyRange.BP_EnemyRange_C" (`SceneComponent.K2_GetComponentToWorld` (`self.spawn2`)) "Undefined" "MultiplyWithRoot" null null))
            (`KismetArrayLibrary.Array_Add` (`self.SpawnedEnemies`) _returnvalue_2)))))))

(event `IntentarMelee`
  (bind _returnvalue (`GameplayStatics.GetPlayerCharacter` 0))
  (if (`self.bJugadorEnMelee`) :!label _label_2
    (set `self.bJugadorEnMelee` false)
    (`self.LaunchCharacter` _returnvalue (10.0 10.0 50.0) false false)
    (`GameplayStatics.ApplyDamage` _returnvalue (`self.DanoMelee`))))

(event `self.Sphere.OnComponentEndOverlap`
  (params (OverlappedComponent :type "PrimitiveComponent Object Reference") (OtherActor :type "Actor Object Reference") (OtherComp :type "PrimitiveComponent Object Reference") (OtherBodyIndex :type Integer))
  (set `self.bJugadorEnMelee` false))

(event `CustomEvent`
  (params (OverlappedComponent :type "PrimitiveComponent Object Reference") (OtherActor :type "Actor Object Reference") (OtherComp :type "PrimitiveComponent Object Reference") (OtherBodyIndex :type Integer) (bFromSweep :type Boolean) (SweepResult :type "HitResult Structure (by ref)"))
  (goto _label_2))

(fn `UserConstructionScript`)