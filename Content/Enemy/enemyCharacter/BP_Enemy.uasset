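; BP_Enemy is an enemy that registers as a level objective and reports completion when killed.
; It faces the player every tick and, once the player comes within range, permanently chases via AIMoveTo reissued each tick.
; Damage plays hit effects and removes at most one HP, with a DoOnce and delay throttling hits until HP equals zero.
; Overlapping its sphere launches and damages the player.
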(event `self.ReceiveTick`
  (params (DeltaSeconds :type "Float (single-precision)"))
  (`self.K2_SetActorRotation` (`KismetMathLibrary.FindLookAtRotation` (`self.K2_GetActorLocation`) (`self.K2_GetActorLocation` (`self.Player`))))
  (if (`self.IsChasing`)
    (`|AIMoveTo` self (0.0 0.0 0.0) (`self.Player`) 100.0)
    (elif (<= (`self.GetDistanceTo` (`self.Player`)) 2600.0)
      (set `self.IsChasing` true))))

(event `self.ReceiveBeginPlay`
  (bind _returnvalue (`GameplayStatics.GetActorOfClass` "/Game/Character/BP_Player.BP_Player_C"))
  (set `self.Player` _returnvalue)
  (bind _outactors (`GameplayStatics.GetAllActorsWithInterface` "/Game/Features/LevelManager/BPI_LevelManager.BPI_LevelManager_C"))
  (message `/Game/Features/LevelManager/BPI_LevelManager.ObjectiveRegistered` (`|GetArrayItem` _outactors)))

(event `SpawnHit`
  (`NiagaraFunctionLibrary.SpawnSystemAtLocation` "/Game/SlashTrail_SoftTofu/Niagara/Dark/NS_Hit_Dark_OnceCopy.NS_Hit_Dark_OnceCopy" (`SceneComponent.K2_GetComponentLocation` (`self.Idle`)))
  (`GameplayStatics.PlaySound2D` "/Game/Character/art/_impacto._impacto" 1.0 1.0 0.0 null null))

(event `self.ReceiveAnyDamage`
  (params (Damage :type "Float (single-precision)") (DamageType :type "DamageType Object Reference") (InstigatedBy :type "Controller Object Reference") (DamageCauser :type "Actor Object Reference"))
  (`/Engine/EditorBlueprintResources/StandardMacros.DoOnce` false :!label _label
    (:`Completed`
      (`self.SpawnHit`)
      (bind _output_get (set `self.HP` (- (`self.HP`) (`KismetMathLibrary.FClamp` Damage))))
      (`KismetSystemLibrary.PrintString` (`KismetStringLibrary.Conv_DoubleToString` _output_get))
      (if (== _output_get 0.0)
        (bind _outactors (`GameplayStatics.GetAllActorsWithInterface` "/Game/Features/LevelManager/BPI_LevelManager.BPI_LevelManager_C"))
        (message `/Game/Features/LevelManager/BPI_LevelManager.ObjectiveCompleted` (`|GetArrayItem` _outactors))
        (`KismetSystemLibrary.Delay` 0.2)
        (`self.K2_DestroyActor`)
        (else
          (`KismetSystemLibrary.Delay` 0.2)
          (goto _label :!via `Reset`))))))

(event `self.Sphere.OnComponentBeginOverlap`
  (params (OverlappedComponent :type "PrimitiveComponent Object Reference") (OtherActor :type "Actor Object Reference") (OtherComp :type "PrimitiveComponent Object Reference") (OtherBodyIndex :type Integer) (bFromSweep :type Boolean) (SweepResult :type "HitResult Structure (by ref)"))
  (bind _returnvalue (`GameplayStatics.GetPlayerCharacter` 0))
  (if (== OtherActor _returnvalue)
    (`self.LaunchCharacter` _returnvalue (10.0 10.0 40.0) false false)
    (`GameplayStatics.ApplyDamage` _returnvalue 10.0)))

(fn `UserConstructionScript`)